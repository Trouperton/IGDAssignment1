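; Player controller that maps input to the controlled pawn for forward movement and turning, fires a Gun and quits the game.
; Movement follows the control rotation's yaw only, and turning scales the axis by the frame time cached on Tick.
; Tick also replays a camera shake every frame on player controller 0, using delta time as its scale.
; Fire calls the Gun reference only when it is valid.
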(event `self.ReceiveTick`
  (params (DeltaSeconds :type "Float (single-precision)"))
  (bind _output_get (set `self.DeltaTime` DeltaSeconds))
  (`self.ClientStartCameraShake` :`self` (`GameplayStatics.GetPlayerController` 0) :`Shake` "/Game/Blueprints/Cameras/CameraShakeOne.CameraShakeOne_C" :`Scale` _output_get))

(event `InputAxis|MoveForward`
  (params (AxisValue :type "Float (single-precision)"))
  (bind _returnvalue (`self.K2_GetPawn`))
  (`Pawn.AddMovementInput` _returnvalue (`KismetMathLibrary.GetForwardVector` (`KismetMathLibrary.MakeRotator` 0.0 0.0 (.yaw (`Pawn.GetControlRotation` _returnvalue)))) AxisValue false))

(event `InputAxis|Turn`
  (params (AxisValue :type "Float (single-precision)"))
  (`Pawn.AddControllerYawInput` (`self.K2_GetPawn`) (* AxisValue (`self.DeltaTime`) 1.2)))

(event `InputAction|Fire`
  (params (Key :type "Key Structure"))
  (bind _gun (`self.gun`))
  (:`Pressed`
    (if (`KismetSystemLibrary.IsValid` _gun)
      (`/Game/Blueprints/Gun_BP.Fire` _gun))))

(event `InputAction|QuitKey`
  (params (Key :type "Key Structure"))
  (:`Pressed`
    (`KismetSystemLibrary.QuitGame` self "Quit")))

(fn `UserConstructionScript`)