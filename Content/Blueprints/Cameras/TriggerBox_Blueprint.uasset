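; Trigger volume Blueprint that switches the player's view to an assigned camera when the player walks into it.
; On collision overlap it prints a debug message naming the entering actor and the trigger.
; If that actor is player 0's pawn, the player controller sets its view target to CameraTriggered.
; There is no end-overlap handling, so the trigger does not restore the previous view on exit.
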(event `self.CollisionComponent.OnComponentBeginOverlap`
  (params (OverlappedComponent :type "PrimitiveComponent Object Reference") (OtherActor :type "Actor Object Reference") (OtherComp :type "PrimitiveComponent Object Reference") (OtherBodyIndex :type Integer) (bFromSweep :type Boolean) (SweepResult :type "HitResult Structure (by ref)"))
  (`KismetSystemLibrary.PrintString` (`KismetStringLibrary.Concat_StrStr` (`KismetStringLibrary.Conv_ObjectToString` OtherActor) " entered " (`KismetStringLibrary.Conv_ObjectToString` self)))
  (if (== (`GameplayStatics.GetPlayerPawn` 0) OtherActor)
    (`PlayerController.SetViewTargetWithBlend` (`GameplayStatics.GetPlayerController` 0) (`self.CameraTriggered`) 0.0 "VTBlend_Linear" 0.0 false)))

(fn `UserConstructionScript`)