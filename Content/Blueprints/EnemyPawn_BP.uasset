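; Enemy pawn that chases the player once triggered and quits the game when it catches the player-controlled MainCharacter.
; Entering TriggerSphere stores the character, destroys the sphere and enables following after a short delay; only then can an actor overlap end the game.
; Tick yaws toward player pawn 0, not the stored CharacterToFollow, and steps forward by Speed each frame without delta-time scaling.
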(event `self.ReceiveActorBeginOverlap`
  (params (OtherActor :type "Actor Object Reference"))
  (if (`KismetSystemLibrary.IsValid` (`self.TriggerSphere`))
    _
    (elif (`self.Following`)
      (bind _asmain_character (cast `/Game/Blueprints/MainCharacter` OtherActor))
      (cast `PlayerController` (`self.GetController` _asmain_character))
      (`KismetSystemLibrary.QuitGame` null "Quit"))))

(event `self.TriggerSphere.OnComponentBeginOverlap`
  (params (OverlappedComponent :type "PrimitiveComponent Object Reference") (OtherActor :type "Actor Object Reference") (OtherComp :type "PrimitiveComponent Object Reference") (OtherBodyIndex :type Integer) (bFromSweep :type Boolean) (SweepResult :type "HitResult Structure (by ref)"))
  (bind _asmain_character (cast `/Game/Blueprints/MainCharacter` OtherActor))
  (set `self.Character to follow` _asmain_character)
  (`ActorComponent.K2_DestroyComponent` (`self.TriggerSphere`))
  (`KismetSystemLibrary.Delay` 0.2)
  (set `self.Following` true))

(event `self.ReceiveTick`
  (params (DeltaSeconds :type "Float (single-precision)"))
  (bind _returnvalue (`KismetMathLibrary.MakeRotator` 0.0 0.0 (.yaw (`KismetMathLibrary.FindLookAtRotation` (`self.K2_GetActorLocation`) (`self.K2_GetActorLocation` (`GameplayStatics.GetPlayerPawn` 0))))))
  (if (`self.Following`)
    (`self.K2_SetActorLocationAndRotation` (+ (`self.K2_GetActorLocation`) (* (`KismetMathLibrary.GetForwardVector` _returnvalue) (`self.Speed`))) _returnvalue)))

(fn `UserConstructionScript`)