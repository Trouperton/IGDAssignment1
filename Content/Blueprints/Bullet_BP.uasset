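; Bullet Blueprint that destroys an enemy pawn on contact and expires ten seconds after spawning.
; On overlap it prints the other actor's name, then casts it to EnemyPawn_BP and destroys both that pawn and itself.
; A delayed quit-game call follows the bullet's self-destruction, so that latent step is unlikely to run.
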(event `self.ReceiveBeginPlay`
  (`KismetSystemLibrary.Delay` 10.0)
  (`self.K2_DestroyActor`))

(event `self.ReceiveActorBeginOverlap`
  (params (OtherActor :type "Actor Object Reference"))
  (`KismetSystemLibrary.PrintString` (`KismetSystemLibrary.GetDisplayName` OtherActor))
  (bind _asenemy_pawn_bp (cast `/Game/Blueprints/EnemyPawn_BP` OtherActor))
  (`self.K2_DestroyActor` _asenemy_pawn_bp)
  (`self.K2_DestroyActor`)
  (`KismetSystemLibrary.Delay` 1.0)
  (`KismetSystemLibrary.QuitGame` (`GameplayStatics.GetPlayerController` 0) "Quit"))

(fn `UserConstructionScript`)